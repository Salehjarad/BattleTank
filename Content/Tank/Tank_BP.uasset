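; Tank Blueprint that registers its aiming parts and handles orbit camera input.
; On BeginPlay it passes its Turret and Barrel components to setter functions not defined in this graph.
; The Azimuth axis yaws AzimuthGimbal, while AimAzimuth, despite its name, pitches the SpringArm.
; Both rotations are local and scaled by world delta seconds and fixed speeds, keeping camera motion frame-rate independent.
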(event `self.ReceiveBeginPlay`
  (`self.SetTurrentComponent` (`self.Turret`))
  (`self.SetBarrelComponent` (`self.Barrel`)))

(event `InputAxis|Azimuth`
  (params (AxisValue :type "Float (single-precision)"))
  ;[1 1 1] Camera Input Binding
  (`SceneComponent.K2_AddLocalRotation` (`self.Azimuth_Gimbal`) (`KismetMathLibrary.MakeRotator` 0.0 0.0 (* AxisValue (`GameplayStatics.GetWorldDeltaSeconds`) 100.0)) false false))

(event `InputAxis|AimAzimuth`
  (params (AxisValue :type "Float (single-precision)"))
  ;[1 1 1] Camera Input Binding
  (`SceneComponent.K2_AddLocalRotation` (`self.SpringArm`) (`KismetMathLibrary.MakeRotator` 0.0 (* AxisValue (`GameplayStatics.GetWorldDeltaSeconds`) 80.0)) false false))

(fn `UserConstructionScript`)